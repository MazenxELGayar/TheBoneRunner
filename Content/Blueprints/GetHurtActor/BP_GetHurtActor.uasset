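; BP_GetHurtActor is an actor with health that can take damage, heal, report its health and deal damage to others.
; Attack runs a single box trace by object type with timed debug drawing, then ApplyHit sends an ApplyDamage message to the hit actor.
; ApplyDamage subtracts HP and returns whether it is dead, while Heal clamps HP between zero and MaxHp.
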(fn ConstructionScript)

(fn ApplyHit
  (params (HitResult :type Hit%20Result%20Structure) (WasHit :type Boolean) (Damage :type Float%20%28double-precision%29))
  (bind _isdead (Class|BPIGetHurt|ApplyDamage(Message) (.HitActor (Collision|BreakHitResult HitResult)) Damage))
  (return HitResult WasHit _isdead))

(fn ApplyDamage
  (params (Damage :type Float%20%28double-precision%29))
  (Variables|HP|SetHP (- (Variables|HP|GetHP) Damage))
  (bind _isdead (CallFunction|IsDead))
  (return _isdead))

(fn Attack
  (params (Damage :type Float%20%28double-precision%29) (BoxTraceStart :type Vector :default "0, 0, 0") (BoxTraceEnd :type Vector :default "0, 0, 0") (TraceExtent :type Vector :default "0, 0, 0") (TraceRotator :type Rotator :default "0, 0, 0") (ObjectTypes :type Array%20of%20EObjectTypeQuery%20Enums :default "ObjectTypeQuery1"))
  (bind (_outhit _returnvalue) (Class|KismetSystemLibrary|BoxTraceSingleforObjects BoxTraceStart BoxTraceEnd TraceExtent TraceRotator ObjectTypes false 0 "ForDuration" true "(R=1.000000,G=0.000000,B=0.000000,A=1.000000)" "(R=0.000000,G=1.000000,B=0.000000,A=1.000000)" 2.0))
  (if _returnvalue
    (bind (_hitresultoutput _washitoutput _died_) (CallFunction|ApplyHit _outhit _returnvalue Damage))
    (return _hitresultoutput _washitoutput _died_)
    (else
      (return _outhit _returnvalue false))))

(fn GetHealth
  (return (Variables|HP|GetHP) (Variables|HP|GetMaxHp)))

(fn GetHealthPercent
  (return (Math|Float|SafeDivide (Variables|HP|GetHP) (Variables|HP|GetMaxHp)) (Variables|HP|GetHP) (Variables|HP|GetMaxHp)))

(fn Heal
  (params (HealAmount :type Float%20%28double-precision%29))
  (bind _output_get (Variables|HP|SetHP (Math|Float|Clamp(Float) (+ HealAmount (Variables|HP|GetHP)) 0.0 (Variables|HP|GetMaxHp))))
  (return _output_get))

(fn IsDead
  (return (<= (Variables|HP|GetHP) 0.0)))