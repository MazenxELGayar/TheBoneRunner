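; BP_EnemyBase is a base enemy character that adds an overhead-style health bar widget to its parent's health logic.
; It caches the WBP_EnemyHealthBar on BeginPlay and refreshes it with the health percentage after parent damage or heal calls.
; Delayed destruction hides the bar, then calls the parent, only if the widget is valid.
; Helper functions move the enemy along its forward vector and rotate it 180 degrees.
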(event EventBeginPlay
  (|CallParentFunction)
  (bind _aswbp_enemy_health_bar (Utilities|Casting|CastToWBP_EnemyHealthBar (UserInterface|GetUserWidgetObject (Variables|Default|GetHealthbarWidget))))
  (Variables|Default|SetAs%20WBP%20Enemy%20Health%20Bar _aswbp_enemy_health_bar))

(event Collision|EventActorBeginOverlap
  (params (OtherActor :type Actor%20Object%20Reference)))

(event EventTick
  (params (DeltaSeconds :type Float%20%28single-precision%29)))

(event EventDestroyActorAfterDelay
  (params (Delay :type Float%20%28double-precision%29))
  (bind _as_wbp_enemy_health_bar (Variables|Default|GetAs%20WBP%20Enemy%20Health%20Bar)
    (:then
      (Widget|SetVisibility _as_wbp_enemy_health_bar "Hidden")
      (|CallParentFunction Delay))
    (:else)))

(fn ConstructionScript)

(fn Move
  (Pawn|Input|AddMovementInput (Transformation|GetActorForwardVector) 1.0 false))

(fn RotateCharacter
  (Transformation|SetActorRotation (Math|Rotator|CombineRotators (Transformation|GetActorRotation) "0.000000,180.000000,0.000000")))

(fn CharApplyDamagetoHealth
  (params (Enemy%20Damage :type Float%20%28double-precision%29))
  (|CallParentFunction Enemy%20Damage)
  (CallFunction|UpdateHealthBar))

(fn UpdateHealthBar
  (Default|UpdateHealth (Variables|Default|GetAs%20WBP%20Enemy%20Health%20Bar) (.Percent (CallFunction|CharGetHealthPercent))))

(fn CharHealCharacter
  (params (Heal%20Amount :type Float%20%28double-precision%29))
  (bind _newhp (|CallParentFunction Heal%20Amount))
  (CallFunction|UpdateHealthBar)
  (return _newhp))