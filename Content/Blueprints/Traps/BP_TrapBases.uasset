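; Base trap Blueprint that deals repeated damage to a character.
; StartDamagingPlayer casts the given actor to BP_CharacterBase, stores it as the target, damages it immediately, then starts a looping timer at HurtingInterval.
; Each tick of that timer passes TrapDamage and the original hit to CharApplyDamageWithAnimations without disabling movement, provided the target is valid.
; StopDamaging clears the timer; nothing in this graph triggers either start or stop.
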(event Custom|StartDamagingPlayer
  (params (Actor :type Actor%20Object%20Reference) (Hit :type Hit%20Result%20Structure))
  (bind _asbp_character_base (Utilities|Casting|CastToBP_CharacterBase Actor)
    (:then
      (Variables|Default|SetTargetPlayer _asbp_character_base)
      (CallFunction|DamagePlayer)
      (bind _returnvalue (Utilities|Time|SetTimerbyEvent (delegate Custom|DamagePlayer) (Variables|Default|GetHurtingInterval) true))
      (Variables|Default|SetTimerHandler _returnvalue))
    (:CastFailed
      (Development|PrintString "FAILED HABIBI"))))

(event Custom|DamagePlayer
  (bind _targetplayer (Variables|Default|GetTargetPlayer)
    (:then
      (Default|CharApplyDamagewithAnimations _targetplayer (Variables|Default|GetTrapDamage) (stale Custom|StartDamagingPlayer Hit) false))
    (:else)))

(event Custom|StopDamaging
  (Utilities|Time|ClearandInvalidateTimerbyHandle (Variables|Default|GetTimerHandler)))

(fn ConstructionScript)