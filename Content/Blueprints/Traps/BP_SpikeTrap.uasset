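; Spike trap Blueprint with a sprite that damages on overlap and grows visibly bloodier as it is triggered.
; Overlap begin calls StartDamagingPlayer, raises a clamped three-stage BloodLevel and refreshes the sprite, while overlap end calls StopDamaging.
; SetRandomSprite picks a random sprite from the normal, semi-bloody or bloody set for that level, and also runs in the construction script for initial variation.
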(event OnComponentBeginOverlap(Sprite)
  (params (OverlappedComponent :type Primitive%20Component%20Object%20Reference) (OtherActor :type Actor%20Object%20Reference) (OtherComp :type Primitive%20Component%20Object%20Reference) (OtherBodyIndex :type Integer) (bFromSweep :type Boolean) (SweepResult :type Hit%20Result%20Structure%20%28by%20ref%29))
  (CallFunction|StartDamagingPlayer OtherActor SweepResult)
  (Variables|Default|SetBloodLevel (Math|Integer|Clamp(Integer) (+ (Variables|Default|GetBloodLevel) 1) 0 2))
  (CallFunction|SetRandomSprite))

(event OnComponentEndOverlap(Sprite)
  (params (OverlappedComponent :type Primitive%20Component%20Object%20Reference) (OtherActor :type Actor%20Object%20Reference) (OtherComp :type Primitive%20Component%20Object%20Reference) (OtherBodyIndex :type Integer))
  (CallFunction|StopDamaging))

(event EventBeginPlay)

(fn ConstructionScript
  (CallFunction|SetRandomSprite))

(fn SetRandomSprite
  (Rendering|Components|Sprite|SetSprite (Variables|Default|GetSprite) (.OutItem (Utilities|Array|Random (Utilities|Select :Index (Variables|Default|GetBloodLevel) :Option%200 (Variables|Default|GetNormalSpikes) :Option%201 (Variables|Default|GetSemiBlodySpikes) :Option%202 (Variables|Default|GetBlodySpikes))))))