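; Behavior Tree decorator that checks whether the AI pawn's combat target is within attack range.
; It reads the CombatTarget actor from the Blackboard and compares the pawn's distance to it against the MinLocationToAttack Blackboard float, passing at or below that value.
; An invalid target fails the check.
; Both outcomes print on-screen debug messages, keyed by actor name.
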(fn PerformConditionCheckAI
  (params (OwnerController :type AI%20Controller%20Object%20Reference) (ControlledPawn :type Pawn%20Object%20Reference))
  (bind _combattarget (Variables|Default|GetCombatTarget))
  (bind _returnvalue (AI|BehaviorTree|GetBlackboardValueasActor _combattarget))
  (Utilities|IsValid _returnvalue
    (:Is%20Valid
      (Variables|Default|SetValidatedActor _returnvalue)
      (Variables|Default|SetDistance (.Distance (CallFunction|InAttackingDistance ControlledPawn (Variables|Default|GetValidatedActor))))
      (Variables|Default|SetInAttackingDistanceValue (.isInAttackingDistance (CallFunction|InAttackingDistance ControlledPawn (Variables|Default|GetValidatedActor))))
      (CallFunction|LogAttackDetails ControlledPawn)
      (return (Variables|Default|GetInAttackingDistanceValue)))
    (:Is%20Not%20Valid
      (CallFunction|LogFailure ControlledPawn)
      (return false))))

(fn InAttackingDistance
  (params (self2 :type Actor%20Object%20Reference) (OtherActor :type Actor%20Object%20Reference))
  (bind _returnvalue (Transformation|GetDistanceTo self2 OtherActor))
  (return (<= _returnvalue (Class|BTFunctionLibrary|GetBlackboardValueasFloat (Variables|Default|GetMinLocationToAttack))) _returnvalue))

(fn LogAttackDetails
  (params (ControlledPawn :type Pawn%20Object%20Reference))
  (Development|PrintString (Utilities|String|Append (Utilities|GetDisplayName (Variables|Default|GetValidatedActor)) " is in Attacking Distance?" (Utilities|GetDisplayName ControlledPawn) " (" (Utilities|String|ToString(Float) (Variables|Default|GetDistance)) " - " (Utilities|String|ToString(Boolean) (Variables|Default|GetInAttackingDistanceValue)) ")") true true "(R=0.000000,G=0.660000,B=1.000000,A=1.000000)" 5.0 (Utilities|String|StringToName (Utilities|String|Append (Utilities|GetDisplayName (Variables|Default|GetValidatedActor)) "AttackingDistance" (Utilities|GetDisplayName ControlledPawn)))))

(fn LogFailure
  (params (Object :type Object%20Object%20Reference))
  (bind _returnvalue (Utilities|GetDisplayName Object))
  (Development|PrintString (Utilities|String|Append _returnvalue " Couldn't find player") true true "(R=0.000000,G=0.660000,B=1.000000,A=1.000000)" 2.0 (Utilities|String|StringToName (Utilities|String|Append _returnvalue "ShouldAttack"))))