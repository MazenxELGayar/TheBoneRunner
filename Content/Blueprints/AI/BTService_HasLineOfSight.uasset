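; Behavior Tree service that tracks how long an enemy AI has been without line of sight to its combat target.
; On tick, it caches the BP_EnemyController and its TargetCharacter, writes the CombatTarget blackboard key, and prints debug messages.
; It then runs LineOfSightTo, resetting TimeSinceLostLineOfSight when visible or otherwise adding the blackboard's CheckLineOfSightInterval instead of measured delta time.
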(event EventReceiveTickAI
  (params (OwnerController :type AI%20Controller%20Object%20Reference) (ControlledPawn :type Pawn%20Object%20Reference) (DeltaSeconds :type Float%20%28single-precision%29))
  (CallFunction|EnsureAIControlllerValid OwnerController)
  (bind _target_character (Variables|Default|GetTarget%20Character)
    (:then
      (CallFunction|SetLineOfSight (Controller|LineOfSightTo (Variables|Default|GetEnemyController) _target_character "0, 0, 0" false)))
    (:else)))

(fn EnsureAIControlllerValid
  (params (AI%20Controller :type AI%20Controller%20Object%20Reference))
  (Variables|Default|GetEnemyController
    (:then
      (Variables|Default|GetTarget%20Character
        (:then)
        (:else
          (CallFunction|SetTargetCharacter))))
    (:else
      (bind _asbp_enemy_controller (Utilities|Casting|CastToBP_EnemyController AI%20Controller)
        (:then
          (Variables|Default|SetEnemyController _asbp_enemy_controller)
          (CallFunction|SetTargetCharacter))
        (:CastFailed
          (Development|PrintString "Cast to enemy controller failed"))))))

(fn SetLineOfSight
  (params (RestTimeSinceLostLineOfSight :type Boolean))
  (Class|BTFunctionLibrary|SetBlackboardValueasFloat (Variables|Default|GetTimeSinceLostLineOfSight) (Math|Float|SelectFloat 0.0 (+ (Class|BTFunctionLibrary|GetBlackboardValueasFloat (Variables|Default|GetTimeSinceLostLineOfSight)) (Class|BTFunctionLibrary|GetBlackboardValueasFloat (Variables|Default|GetCheckLineOfSightInterval))) RestTimeSinceLostLineOfSight)))

(fn SetTargetCharacter
  (bind _enemycontroller (Variables|Default|GetEnemyController))
  (bind _returnvalue (Utilities|GetDisplayName _enemycontroller))
  (bind _targetcharacter (Variables|/Game/Blueprints/AI/BP_EnemyController.BP_EnemyController_C|GetTargetCharacter (Variables|Default|GetEnemyController))
    (:then
      (Variables|Default|SetTarget%20Character _targetcharacter)
      (bind _target_character (Variables|Default|GetTarget%20Character)
        (:then
          (Class|BTFunctionLibrary|SetBlackboardValueasObject (Variables|Default|GetCombatTarget) _target_character)
          (Development|PrintString (Utilities|String|Append _returnvalue " Combat Target Was Set To  " (Utilities|GetDisplayName (Variables|Default|GetTarget%20Character))) true true "(R=0.092641,G=1.000000,B=0.121956,A=1.000000)" 5.0 (Utilities|String|StringToName (Utilities|String|Append _returnvalue "CombatTargetFound"))))
        (:else
          (Development|PrintString (Utilities|String|Append (Utilities|GetDisplayName (Variables|Default|GetEnemyController)) " Combat Target Is Not An Actor") true true "(R=1.000000,G=0.053293,B=0.000000,A=1.000000)" 5.0 (Utilities|String|StringToName (Utilities|String|Append (Utilities|GetDisplayName (Variables|Default|GetEnemyController)) "CombatTargetNotFound")) :!label _label))))
    (:else
      (goto _label))))