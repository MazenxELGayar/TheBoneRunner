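; Behavior tree task that picks a random location for an AI pawn and writes it to a Blackboard vector key, then finishes successfully.
; A helper function queries reachable navigation points within a fixed radius of the pawn.
; It keeps the pawn's current Y and takes only X and Z from the query, so the composed target is not guaranteed reachable.
; A debug sphere draw is left disconnected.
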(event EventReceiveExecuteAI
  (params (OwnerController :type AI%20Controller%20Object%20Reference) (ControlledPawn :type Pawn%20Object%20Reference))
  (Variables|Default|SetRandom%20Location (CallFunction|GetRandomReachableLocation ControlledPawn))
  (AI|BehaviorTree|SetBlackboardValueasVector (Variables|Default|GetBBKeyLocation) (Variables|Default|GetRandom%20Location))
  (AI|BehaviorTree|FinishExecute true))

(fn GetRandomReachableLocation
  (params (Actor :type Actor%20Object%20Reference))
  (bind _returnvalue (Transformation|GetActorLocation Actor))
  (bind _randomlocation (AI|Navigation|GetRandomReachablePointinRadius _returnvalue 2.5e+03 0 0))
  (return (Math|Vector|MakeVector (.x _randomlocation) (.Y (Math|Vector|BreakVector _returnvalue)) (.z _randomlocation))))