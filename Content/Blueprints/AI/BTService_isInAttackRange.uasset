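; Behavior tree service that tells an AI pawn whether its combat target is within attack and chase range.
; Each tick, if the time since line of sight was lost is within the blackboard's reset limit, it validates the blackboard combat target and measures the distance to it.
; It writes that distance, plus attack and chase booleans compared against blackboard thresholds, back to the blackboard.
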(event EventReceiveTickAI
  (params (OwnerController :type AI%20Controller%20Object%20Reference) (ControlledPawn :type Pawn%20Object%20Reference) (DeltaSeconds :type Float%20%28single-precision%29))
  (if (CallFunction|HasLineOfSight)
    (CallFunction|CaclulateandSetinAttackingDistance ControlledPawn)))

(fn LogFailure
  (params (Object :type Object%20Object%20Reference))
  (bind _returnvalue (Utilities|GetDisplayName Object))
  (Development|PrintString (Utilities|String|Append _returnvalue " Couldn't find player") true true "(R=0.000000,G=0.660000,B=1.000000,A=1.000000)" 2.0 (Utilities|String|StringToName (Utilities|String|Append _returnvalue "ShouldAttack"))))

(fn LogAttackDetails
  (params (ControlledPawn :type Pawn%20Object%20Reference))
  (Development|PrintString (Utilities|String|Append (Utilities|GetDisplayName (Variables|Default|GetValidatedActor)) " - " (Utilities|GetDisplayName ControlledPawn) " D:" (Utilities|String|ToString(Float) (Variables|Default|GetDistance)) "  is in Attacking Distance? " (Utilities|String|ToString(Boolean) (Variables|Default|GetInAttackingDistanceValue)) "" " -  is in Chasing Distance? " (Utilities|String|ToString(Boolean) (Variables|Default|GetIn%20Chase%20Distance))) true true "(R=0.000000,G=0.660000,B=1.000000,A=1.000000)" 5.0 (Utilities|String|StringToName (Utilities|String|Append (Utilities|GetDisplayName (Variables|Default|GetValidatedActor)) "AttackingDistance" (Utilities|GetDisplayName ControlledPawn)))))

(fn SetDistanceandFlags
  (params (ControlledPawn :type Actor%20Object%20Reference) (CombatTarget :type Actor%20Object%20Reference))
  (CallFunction|CaculateDistance ControlledPawn CombatTarget)
  (CallFunction|InAttackDistance (Variables|Default|GetDistance))
  (CallFunction|InChaseDistance (Variables|Default|GetDistance))
  (return (Variables|Default|GetInAttackingDistanceValue) (Variables|Default|GetDistance) (Variables|Default|GetIn%20Chase%20Distance)))

(fn CaclulateandSetinAttackingDistance
  (params (ControlledPawn :type Pawn%20Object%20Reference))
  (bind _combattarget (Variables|Default|GetCombatTarget))
  (bind _returnvalue (AI|BehaviorTree|GetBlackboardValueasActor _combattarget))
  (Utilities|IsValid _returnvalue
    (:Is%20Valid
      (Variables|Default|SetValidatedActor _returnvalue)
      (CallFunction|SetDistanceandFlags ControlledPawn (Variables|Default|GetValidatedActor)))))

(fn InAttackDistance
  (params (Distance :type Float%20%28double-precision%29))
  (Variables|Default|SetInAttackingDistanceValue (<= Distance (Class|BTFunctionLibrary|GetBlackboardValueasFloat (Variables|Default|GetMinLocationToAttack))))
  (Class|BTFunctionLibrary|SetBlackboardValueasBool (Variables|Default|GetInAttackingDistanceKey) (Variables|Default|GetInAttackingDistanceValue))
  (return (Variables|Default|GetInAttackingDistanceValue)))

(fn InChaseDistance
  (params (Distance :type Float%20%28double-precision%29))
  (Variables|Default|SetIn%20Chase%20Distance (<= Distance (Class|BTFunctionLibrary|GetBlackboardValueasFloat (Variables|Default|GetMaxDistanceToChase))))
  (Class|BTFunctionLibrary|SetBlackboardValueasBool (Variables|Default|GetInChaseDistanceKey) (Variables|Default|GetIn%20Chase%20Distance))
  (return (Variables|Default|GetIn%20Chase%20Distance)))

(fn HasLineOfSight
  (return (<= (Class|BTFunctionLibrary|GetBlackboardValueasFloat (Variables|Default|GetTimeSinceLostLineOfSight)) (Class|BTFunctionLibrary|GetBlackboardValueasFloat (Variables|Default|GetMaxLostLineOfSightUntilReset)))))

(fn CaculateDistance
  (params (ControlledPawn :type Actor%20Object%20Reference) (CombatTarget :type Actor%20Object%20Reference))
  (Variables|Default|SetDistance (Transformation|GetDistanceTo ControlledPawn CombatTarget))
  (Class|BTFunctionLibrary|SetBlackboardValueasFloat (Variables|Default|GetDistanceToCombatTarget) (Variables|Default|GetDistance))
  (return (Variables|Default|GetDistance)))