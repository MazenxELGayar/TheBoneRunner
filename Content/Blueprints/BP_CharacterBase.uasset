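; Base 2D character using PaperZD, providing health, healing, melee attacks, hurt reactions and death.
; Attacks cycle through an animation array and lock out until a delay fed by the animation override's return value ends.
; A separate attack function box-traces between two components and damages any hit BP_CharacterBase.
; Taking damage blocks attacking and plays a hurt or death override, then either re-enables attacks or destroys the actor after that delay.
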(event Custom|DestroyActorAfterDelay
  (params (Delay :type Float%20%28double-precision%29))
  (Development|PrintString (Utilities|String|ToString(Float) Delay))
  (Utilities|FlowControl|Delay Delay)
  (Actor|DestroyActor))

(event Custom|ResetAttacking
  (params (Delay :type Float%20%28double-precision%29))
  (Utilities|FlowControl|Delay Delay)
  (Variables|Default|SetDisableAttack false))

(event EventBeginPlay)

(event Collision|EventActorBeginOverlap
  (params (OtherActor :type Actor%20Object%20Reference)))

(event EventTick
  (params (DeltaSeconds :type Float%20%28single-precision%29)))

(fn ConstructionScript)

(fn CharApplyHit
  (params (HitResult :type Hit%20Result%20Structure) (WasHit :type Boolean) (Damage :type Float%20%28double-precision%29))
  (bind _asbp_character_base (Utilities|Casting|CastToBP_CharacterBase (.HitActor (Collision|BreakHitResult HitResult))))
  (bind _died_ (CallFunction|CharApplyDamage _asbp_character_base Damage))
  (return HitResult WasHit _died_))

(fn CharPlayAttackAnimation
  (if (not (Variables|Default|GetDisableAttack))
    (Variables|Default|SetDisableAttack true)
    (bind _animationlength (CallFunction|CharPlayAnimation (Utilities|Array|Get(acopy) (Variables|Default|GetAttacks) (Variables|Default|GetAttackIndex)) "DefaultSlot" (Variables|Default|GetAttack%20Play%20Rate) 0.0))
    (CallFunction|CharRestorNextAttackAnimation)
    (CallFunction|ResetAttacking _animationlength)))

(fn CharGetHealthPercent
  (return (Math|Float|SafeDivide (Variables|Default|GetHP) (Variables|Default|GetMaxHp)) (Variables|Default|GetHP) (Variables|Default|GetMaxHp)))

(fn CharGetHealth
  (return (Variables|Default|GetHP) (Variables|Default|GetMaxHp)))

(fn CharIsDead
  (return (<= (Variables|Default|GetHP) 0.0)))

(fn CharAttemptAttack
  (bind (_outhit _returnvalue) (Class|KismetSystemLibrary|BoxTraceSingleforObjects (Transformation|GetWorldLocation (Variables|Default|GetAttackBoxTraceStart)) (Transformation|GetWorldLocation (Variables|Default|GetAttackBoxTraceEnd)) (Variables|Default|GetTrace%20Extent) (Variables|Default|GetTrace%20Rotator) (Variables|Default|GetObject%20Types) false 0 "ForDuration" true "(R=1.000000,G=0.000000,B=0.000000,A=1.000000)" "(R=0.000000,G=1.000000,B=0.000000,A=1.000000)" 2.0))
  (if _returnvalue
    (bind (_hitresultoutput _washitoutput _died_) (CallFunction|CharApplyHit _outhit _returnvalue (Variables|Default|GetDamage)))
    (return _hitresultoutput _washitoutput _died_)
    (else
      (return _outhit _returnvalue false))))

(fn CharApplyDamage
  (params (EnemyDamage :type Float%20%28double-precision%29))
  (Variables|Default|SetDisableAttack true)
  (Variables|Default|SetHP (- (Variables|Default|GetHP) EnemyDamage))
  (bind _isdead (CallFunction|CharIsDead))
  (bind _animationlength (CallFunction|CharPlayAnimation (select _isdead (Variables|Default|GetDeadAnimation) (Variables|Default|GetHurtAnimation)) "HurtOverride" 1.0 0.0))
  (if _isdead
    (CallFunction|DestroyActorAfterDelay _animationlength)
    (else
      (CallFunction|ResetAttacking _animationlength)
      (return _isdead))))

(fn CharHealCharacter
  (params (Heal%20Amount :type Float%20%28double-precision%29))
  (bind _output_get (Variables|Default|SetHP (Math|Float|Clamp(Float) (+ Heal%20Amount (Variables|Default|GetHP)) 0.0 (Variables|Default|GetMaxHp))))
  (return _output_get))

(fn CharRestorNextAttackAnimation
  (Variables|Default|SetAttackIndex (Math|Integer|SelectInt (+ (Variables|Default|GetAttackIndex) 1) 0 (< (+ (Variables|Default|GetAttackIndex) 1) (Utilities|Array|Length (Variables|Default|GetAttacks))))))

(fn CharPlayAnimation
  (params (AnimSequence :type Paper%20ZD%20Anim%20Sequence%20Object%20Reference) (SlotName :type Name :default "DefaultSlot") (PlayRate :type Float%20%28double-precision%29) (StartingPosition :type Float%20%28double-precision%29))
  (bind _animationlength (Class|PaperZDAnimInstance|PlayAnimationOverride (Variables|/Script/PaperZD.PaperZDAnimationComponent|GetAnimInstance (Variables|Default|GetPaperZDAnimation)) AnimSequence SlotName PlayRate StartingPosition))
  (return _animationlength))