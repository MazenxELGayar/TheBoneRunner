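; BP_RedHood is the Red Hood actor Blueprint, exposing damage, healing and health queries.
; Each health function forwards to BPGetHurtActor through message calls and returns its result, so the Blueprint holds no health logic of its own.
; The event graph and construction script are empty.
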(event EventBeginPlay)

(event Collision|EventActorBeginOverlap
  (params (OtherActor :type Actor%20Object%20Reference)))

(event EventTick
  (params (DeltaSeconds :type Float%20%28single-precision%29)))

(fn ConstructionScript)

(fn ApplyDamage
  (params (Damage :type Float%20%28double-precision%29))
  (bind _isdead (Class|BPIGetHurt|ApplyDamage(Message) (Variables|Default|GetBP_GetHurtActor) Damage))
  (return _isdead))

(fn GetHealth
  (bind (_hp _maxhp) (Class|BPIGetHurt|GetHealth(Message) (Variables|Default|GetBP_GetHurtActor)))
  (return _hp _maxhp))

(fn GetHealthPercent
  (bind (_percent _hp _maxhp) (Class|BPIGetHurt|GetHealthPercent(Message) (Variables|Default|GetBP_GetHurtActor)))
  (return _percent _hp _maxhp))

(fn Heal
  (params (HealAmount :type Float%20%28double-precision%29))
  (bind _newhp (Class|BPIGetHurt|Heal(Message) (Variables|Default|GetBP_GetHurtActor) HealAmount))
  (return _newhp))

(fn IsDead
  (bind _isdead (Class|BPIGetHurt|IsDead(Message) (Variables|Default|GetBP_GetHurtActor)))
  (return _isdead))